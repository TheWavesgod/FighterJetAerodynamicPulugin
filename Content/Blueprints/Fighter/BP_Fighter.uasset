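; Player-controlled fighter aircraft pawn that routes flight input into its FlightPhysicsComponent.
; Axes drive stick, rudders, throttle, flaps, brake and wheel steering; actions toggle the flight control system and an engine-running flag.
; V swaps first-person and external cameras, NumPad 3 opens the Demonstration level, and BeginPlay creates a Fighter widget bound to this pawn.
; SetSoundParameters maps physics state to SoundsBP, but its call, like Startup's, is disconnected.
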(event `Key|NumPadThree`
  (params (Key :type "Key Structure"))
  (:`Pressed`
    (`GameplayStatics.OpenLevelBySoftObjectPtr` "/Game/MBP/Maps/Demonstration/Demonstration.Demonstration")))

(event `InputAxis|Brake`
  (params (AxisValue :type "Float (single-precision)"))
  (`FlightPhysicsComponent.SetWheelsBrake` (`self.FlightPhysicsComponent`) (`KismetMathLibrary.SelectFloat` 0.9 0.0 (> AxisValue 0.5))))

(event `InputAxis|LookUp`
  (params (AxisValue :type "Float (single-precision)"))
  (`self.AddControllerPitchInput` AxisValue))

(event `InputAxis|TurnRight`
  (params (AxisValue :type "Float (single-precision)"))
  (`self.AddControllerYawInput` AxisValue))

(event `InputAxis|Flaps`
  (params (AxisValue :type "Float (single-precision)"))
  (`FlightPhysicsComponent.SetFlaps` (`self.FlightPhysicsComponent`) AxisValue))

(event `InputAxis|ThrottleControl`
  (params (AxisValue :type "Float (single-precision)"))
  (`FlightPhysicsComponent.SetAddThruster` (`self.FlightPhysicsComponent`) AxisValue))

(event `InputAction|FlyControlSystemSwitch`
  (params (Key :type "Key Structure"))
  (bind _flightphysicscomponent (`self.FlightPhysicsComponent`))
  (:`Pressed`
    (`FlightPhysicsComponent.SetFlyingControlSystemActivated` _flightphysicscomponent (not (`FlightPhysicsComponent.GetFlyingControlSystemState` _flightphysicscomponent)))))

(event `InputAxis|WheelSteering`
  (params (AxisValue :type "Float (single-precision)"))
  (`FlightPhysicsComponent.SetSteeringWheels` (`self.FlightPhysicsComponent`) AxisValue))

(event `InputAxis|Roll`
  (params (AxisValue :type "Float (single-precision)"))
  (`FlightPhysicsComponent.SetControlStickXAxis` (`self.FlightPhysicsComponent`) AxisValue))

(event `InputAction|Engine`
  (params (Key :type "Key Structure"))
  (:`Pressed`
    (set `self.IsEngineRunning` (not (`self.IsEngineRunning`)))))

(event `InputAxis|Pitch`
  (params (AxisValue :type "Float (single-precision)"))
  (`FlightPhysicsComponent.SetControlStickYAxis` (`self.FlightPhysicsComponent`) AxisValue))

(event `InputAxis|Yaw`
  (params (AxisValue :type "Float (single-precision)"))
  (`FlightPhysicsComponent.SetRudders` (`self.FlightPhysicsComponent`) AxisValue))

(event `Key|V`
  (params (Key :type "Key Structure"))
  (bind _fppcamera (`self.FPPCamera`))
  (bind _camera (`self.Camera`))
  (:`Pressed`
    (`/Engine/EditorBlueprintResources/StandardMacros.FlipFlop`
      (:`A`
        (`ActorComponent.SetActive` _fppcamera true false)
        (`ActorComponent.SetActive` _camera false false))
      (:`B`
        (`ActorComponent.SetActive` _fppcamera false false)
        (`ActorComponent.SetActive` _camera true false)))))

(event `self.ReceiveBeginPlay`
  (`parent.ReceiveBeginPlay`)
  (bind _returnvalue (`|CreateWidget` "/Game/Blueprints/Fighter/Fighter.Fighter_C" (`GameplayStatics.GetPlayerController` 0)))
  (`UserWidget.AddToPlayerScreen` _returnvalue 0)
  (set `/Game/Blueprints/Fighter/Fighter.Fighter` self _returnvalue))

(event `self.ReceiveTick`
  (params (DeltaSeconds :type "Float (single-precision)"))
  (`parent.ReceiveTick` DeltaSeconds))

(fn `SetSoundParameters`
  (bind _flightphysicscomponent (`self.FlightPhysicsComponent`))
  (bind _sounds_bp (`self.Sounds_BP`))
  (`Sounds_F35.SetRPM` _sounds_bp (`FlightPhysicsComponent.GetCurrentThrusterRatio` _flightphysicscomponent))
  (`Sounds_F35.SetSpeed` _sounds_bp (/ (`FlightPhysicsComponent.GetGroundSpeed` _flightphysicscomponent) 0.036))
  (`Sounds_F35.SetPitchRate` _sounds_bp (`FlightPhysicsComponent.GetCurrentGForce` _flightphysicscomponent))
  (`Sounds_F35.SetIsEngineRunning` _sounds_bp (`self.IsEngineRunning`))
  (`Sounds_F35.SetIsPlaneOnLand` _sounds_bp true))

(fn `UserConstructionScript`)